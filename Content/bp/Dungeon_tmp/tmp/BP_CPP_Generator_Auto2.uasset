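; Procedural dungeon generator that builds room floors from the construction script, with an optional reseed of its random stream.
; CreateRooms supplies tile coordinates, which become instanced static meshes on a 200-unit grid.
; Scaled room centers feed a Delaunay triangulation, whose hull-triangle points feed an MST function.
; Corridors are not built: triangle edges are only debug-drawn, MST trace endpoints lack X/Y inputs, and connection-map code is unwired.
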(event `StartGeneration`
  (bind (_returnvalue_x _returnvalue_y _returnvalue_z) (`KismetMathLibrary.BreakVector` (`SceneComponent.K2_GetComponentLocation` (`self.InstancedStaticMeshComponent`))))
  (bind (_returnvalue_x_2 _returnvalue_y_2 _returnvalue_z_2) (`KismetMathLibrary.BreakVector` (`SceneComponent.K2_GetComponentLocation` (`self.InstancedStaticMeshComponent`))))
  (bind (_returnvalue_x_3 _returnvalue_y_3 _returnvalue_z_3) (`KismetMathLibrary.BreakVector` (`SceneComponent.K2_GetComponentLocation` (`self.InstancedStaticMeshComponent`))))
  (`KismetSystemLibrary.FlushPersistentDebugLines`) ; clean debug delaunay lines even if theyre doesnt exists
  (`self.CreateFloorTiles` (`self.Max Loops`) (`self.Room Count`) (`self.Room Size Min`) (`self.Room Size Max`) (`self.Floor Tile Size`) (`self.Min Distance`) (`self.Max Distance`)) ; generating procedural room floor tiles and modeling them
  (for _index (range (+ (`KismetArrayLibrary.Array_LastIndex` (`self.RoomDataArray`)) 1))
    (bind _output_center (break `RoomData` (`|GetArrayItem` (`self.RoomDataArray`) _index)))
    (bind _returnvalue (* _output_center (200.0 200.0)))
    (`KismetArrayLibrary.Array_Set` (`self.RoomDataArray`) _index (make `RoomData` _returnvalue))
    (`KismetArrayLibrary.Array_Add` (`self.RoomCentersList`) _returnvalue))
  (bind _output_get (set `self.triangulated_corridors` (`DelaunayHelper.CreateDelaunayTriangulation` (`self.RoomCentersList`))))
  (for _index_2 (range (+ (`KismetArrayLibrary.Array_LastIndex` (`.HullTriangles` (break `DelaunayMesh` _output_get))) 1))
    ;[1 1 1] DRAWING DEBUG LINE TRACE
    (`|ExecutionSequence`
      (:`then_0`
        (bind _returnvalue_2 (`DelaunayHelper.ConvertTriangleIDToTriangle` (`self.triangulated_corridors`) (`|GetArrayItem` (`.HullTriangles` (break `DelaunayMesh` _output_get)) _index_2)))
        (bind _returnvalue_3 (+ (`KismetMathLibrary.BreakVector2D` (break `DelaunayTriangle` _returnvalue_2)) _returnvalue_x_3))
        (bind _returnvalue_4 (+ (`.Y` (`KismetMathLibrary.BreakVector2D` (break `DelaunayTriangle` _returnvalue_2))) _returnvalue_y_3))
        (`KismetArrayLibrary.Array_Add` (`self.triangle_points_arr`) (`KismetMathLibrary.MakeVector2D` _returnvalue_3 _returnvalue_4))
        (if (`self.ENABLE_DEBUG`)
          (`KismetSystemLibrary.LineTraceSingle` :`Start` (`KismetMathLibrary.MakeVector` _returnvalue_3 _returnvalue_4 _returnvalue_z_3) :`End` (`KismetMathLibrary.MakeVector` (+ (`KismetMathLibrary.BreakVector2D` (`.B` (break `DelaunayTriangle` _returnvalue_2))) _returnvalue_x_3) (+ (`.Y` (`KismetMathLibrary.BreakVector2D` (`.B` (break `DelaunayTriangle` _returnvalue_2)))) _returnvalue_y_3) _returnvalue_z_3) :`TraceChannel` "TraceTypeQuery2" :`DrawDebugType` "Persistent" :`TraceHitColor` (struct :`R` 0.768628 :`B` 0.572549 :`A` 1.0) :`DrawTime` 30.0)))
      (:`then_1`
        (bind _returnvalue_5 (+ (`KismetMathLibrary.BreakVector2D` (`.B` (break `DelaunayTriangle` _returnvalue_2))) _returnvalue_x))
        (bind _returnvalue_6 (+ (`.Y` (`KismetMathLibrary.BreakVector2D` (`.B` (break `DelaunayTriangle` _returnvalue_2)))) _returnvalue_y))
        (`KismetArrayLibrary.Array_Add` (`self.triangle_points_arr`) (`KismetMathLibrary.MakeVector2D` _returnvalue_5 _returnvalue_6))
        (if (`self.ENABLE_DEBUG`)
          (`KismetSystemLibrary.LineTraceSingle` :`Start` (`KismetMathLibrary.MakeVector` _returnvalue_5 _returnvalue_6 _returnvalue_z) :`End` (`KismetMathLibrary.MakeVector` (+ (`KismetMathLibrary.BreakVector2D` (`.C` (break `DelaunayTriangle` _returnvalue_2))) _returnvalue_x) (+ (`.Y` (`KismetMathLibrary.BreakVector2D` (`.C` (break `DelaunayTriangle` _returnvalue_2)))) _returnvalue_y) _returnvalue_z) :`TraceChannel` "TraceTypeQuery2" :`DrawDebugType` "Persistent" :`TraceHitColor` (struct :`R` 0.768628 :`B` 0.572549 :`A` 1.0) :`DrawTime` 30.0)))
      (:`then_2`
        (bind _returnvalue_7 (+ (`KismetMathLibrary.BreakVector2D` (`.C` (break `DelaunayTriangle` _returnvalue_2))) _returnvalue_x_2))
        (bind _returnvalue_8 (+ (`.Y` (`KismetMathLibrary.BreakVector2D` (`.C` (break `DelaunayTriangle` _returnvalue_2)))) _returnvalue_y_2))
        (`KismetArrayLibrary.Array_Add` (`self.triangle_points_arr`) (`KismetMathLibrary.MakeVector2D` _returnvalue_7 _returnvalue_8))
        (if (`self.ENABLE_DEBUG`)
          (`KismetSystemLibrary.LineTraceSingle` :`Start` (`KismetMathLibrary.MakeVector` _returnvalue_7 _returnvalue_8 _returnvalue_z_2) :`End` (`KismetMathLibrary.MakeVector` (+ (`KismetMathLibrary.BreakVector2D` (break `DelaunayTriangle` _returnvalue_2)) _returnvalue_x_2) (+ (`.Y` (`KismetMathLibrary.BreakVector2D` (break `DelaunayTriangle` _returnvalue_2))) _returnvalue_y_2) _returnvalue_z_2) :`TraceChannel` "TraceTypeQuery2" :`DrawDebugType` "Persistent" :`TraceHitColor` (struct :`R` 0.768628 :`B` 0.572549 :`A` 1.0) :`DrawTime` 30.0)))))
  (bind _returnvalue_9 (`self.MST` (`self.triangle_points_arr`) 0 200))
  (for _index_3 (range (+ (`KismetArrayLibrary.Array_LastIndex` _returnvalue_9) 1))
    (if true
      (`KismetSystemLibrary.LineTraceSingle` :`Start` (`KismetMathLibrary.MakeVector` 0.0 0.0 _returnvalue_z_2) :`End` (`KismetMathLibrary.MakeVector` 0.0 0.0 _returnvalue_z_2) :`TraceChannel` "TraceTypeQuery2" :`DrawDebugType` "Persistent" :`TraceColor` (struct :`R` 0.94 :`G` 0.264966 :`A` 1.0) :`TraceHitColor` (struct :`G` 0.077584 :`B` 0.68 :`A` 1.0) :`DrawTime` 30.0))))

(fn `CreateFloorTiles`
  (params (`Max Loops` :type Integer) (RoomCount :type Integer) (RoomSizeMin :type Integer) (RoomSizeMax :type Integer) (FloorTileSize :type Integer) (MinDistance :type Integer) (MaxDistance :type Integer))
  (set `self.MaxLoops` `Max Loops`)
  (`KismetArrayLibrary.Array_Clear` (`self.FloorTilesCords`))
  (`InstancedStaticMeshComponent.ClearInstances` (`self.InstancedStaticMeshComponent`))
  (bind _returnvalue (`self.CreateRooms` RoomCount RoomSizeMin RoomSizeMax FloorTileSize MinDistance MaxDistance))
  (bind _output_get (set `self.FloorTilesCords` _returnvalue))
  (for _index (range (+ (`KismetArrayLibrary.Array_LastIndex` _output_get) 1))
    (bind (_output_x _output_y) (`KismetMathLibrary.BreakVector2D` (`|GetArrayItem` (`self.FloorTilesCords`) _index)))
    (`InstancedStaticMeshComponent.AddInstance` (`self.InstancedStaticMeshComponent`) (`KismetMathLibrary.MakeTransform` (`KismetMathLibrary.MakeVector` (* _output_x 200.0) (* _output_y 200.0))) false)))

(fn `UserConstructionScript`
  (`|ExecutionSequence`
    (:`then_0`
      (if (`self.NewSeed`)
        (set `self.NewSeed` false)
        (set `self.SEED` (`KismetMathLibrary.RandomInteger` 900000))
        (`KismetMathLibrary.SetRandomStreamSeed` (`self.GeneratorStream`) (`self.SEED`))))
    (:`then_1`
      (`self.StartGeneration`))))