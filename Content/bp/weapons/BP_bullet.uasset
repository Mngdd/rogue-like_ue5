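; BP_bullet is a projectile weapon bullet that flies at a supplied velocity and is destroyed on impact.
; On BeginPlay it copies its Velocity variable into the ProjectileMovement component.
; On hit it prints the hit actor's name, spawns an impact particle at the impact point for non-Character targets, then destroys itself.
; It applies no damage, and a hard-coded true branch leaves a debug print unreachable.
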(event `self.ReceiveBeginPlay`
  ;[1 1 1] set custom velocity from input when actor spawns
  (set `MovementComponent.Velocity` (`self.velocity`) (`self.ProjectileMovement`)))

(event `self.ReceiveHit`
  (params (MyComp :type "PrimitiveComponent Object Reference") (Other :type "Actor Object Reference") (OtherComp :type "PrimitiveComponent Object Reference") (bSelfMoved :type Boolean) (HitLocation :type "Vector Structure") (HitNormal :type "Vector Structure") (NormalImpulse :type "Vector Structure") (Hit :type "HitResult Structure (by ref)"))
  (bind (_bblockinghit _binitialoverlap _time _distance _location _impactpoint _normal _impactnormal _physmat _hitactor) (`GameplayStatics.BreakHitResult` Hit))
  (`KismetSystemLibrary.PrintString` (`KismetSystemLibrary.GetDisplayName` _hitactor))
  (if true
    (cast `Character` Other
      (:`then`
        _)
      (:`CastFailed`
        (`GameplayStatics.SpawnEmitterAtLocation` "/Game/PrototypeWeap/FX/P_Impact_01.P_Impact_01" _impactpoint)))
    (`self.K2_DestroyActor`)
    (else
      (`KismetSystemLibrary.PrintString` "Hello"))))

(fn `UserConstructionScript`)