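; Base weapon actor that is picked up, equipped to a player slot, fired, reloaded and dropped, toggling physics and collision by state.
; BeginPlay loads its stats and ammo from DT_weapondata by name.
; Shoot handles single, burst and automatic modes, using a timer to gate and repeat shots and a delayed loop for bursts.
; Bullets and muzzle flashes spawn at the muzzle socket, with velocity aimed at a distant point along the camera's forward vector.
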(event `Shoot`
  (if (and (> (`self.Ammo Mag Curr`) 0) (`self.IsShooting?`) (`KismetStringLibrary.EqualEqual_StrStr` (`|GetEnumeratorNameAsString` (`/Game/bp/BP_player_char.CurrentWeaponSlot` (`self.Player`))) (`self.MySlot`)))
    (if (`self.ShootDelayOver?`)
      (if (`|EnumEquality` (`self.Firemode`) "NewEnumerator0")
        (`/Game/bp/BP_player_char.Play User Animation` (`self.Player`) "fire")
        (bind (_transform_location _velocity _transform_rotation) (`self.calc_vel_and_path`))
        (`|SpawnActorFromClass` "/Game/bp/weapons/BP_bullet.BP_bullet_C" (`KismetMathLibrary.MakeTransform` _transform_location _transform_rotation) "Undefined" "OverrideRootScale" null _velocity null)
        (`|SpawnActorFromClass` "/Game/bp/weapons/BP_MuzzleFlash.BP_MuzzleFlash_C" (`KismetMathLibrary.MakeTransform` _transform_location) "Undefined" "OverrideRootScale" null null)
        (set `self.Ammo Mag Curr` (- (`self.Ammo Mag Curr`) 1))
        (set `self.ShootDelayOver?` false)
        (`KismetSystemLibrary.K2_SetTimer` null "RememberShootDelay" (`self.Firerate`))
        (elif (`|EnumEquality` (`self.Firemode`) "NewEnumerator1")
          (set `self.ShootDelayOver?` false)
          (`KismetSystemLibrary.K2_SetTimer` null "RememberShootDelay" (`self.Burst Delay`))
          (`/Game/bp/ForLoopWithDelay.Loop With Delay and Break` 0 (`self.Burst Amount`) (`self.Firerate`) :!label _label
            (:`Loop Body`
              (`/Game/bp/BP_player_char.Play User Animation` (`self.Player`) "fire")
              (bind (_transform_location_2 _velocity_2 _transform_rotation_2) (`self.calc_vel_and_path`))
              (`|SpawnActorFromClass` "/Game/bp/weapons/BP_bullet.BP_bullet_C" (`KismetMathLibrary.MakeTransform` _transform_location_2 _transform_rotation_2) "Undefined" "OverrideRootScale" null _velocity_2 null)
              (`|SpawnActorFromClass` "/Game/bp/weapons/BP_MuzzleFlash.BP_MuzzleFlash_C" (`KismetMathLibrary.MakeTransform` _transform_location_2) "Undefined" "OverrideRootScale" null null)
              (set `self.Ammo Mag Curr` (- (`self.Ammo Mag Curr`) 1))
              (if (not (and (> (`self.Ammo Mag Curr`) 0) (`KismetStringLibrary.EqualEqual_StrStr` (`|GetEnumeratorNameAsString` (`/Game/bp/BP_player_char.CurrentWeaponSlot` (`self.Player`))) (`self.MySlot`))))
                (goto _label :!via `Break`))))
          (elif (`|EnumEquality` (`self.Firemode`) "NewEnumerator2")
            (`/Game/bp/BP_player_char.Play User Animation` (`self.Player`) "fire")
            (bind (_transform_location_3 _velocity_3 _transform_rotation_3) (`self.calc_vel_and_path`))
            (`|SpawnActorFromClass` "/Game/bp/weapons/BP_bullet.BP_bullet_C" (`KismetMathLibrary.MakeTransform` _transform_location_3 _transform_rotation_3) "Undefined" "OverrideRootScale" null _velocity_3 null)
            (`|SpawnActorFromClass` "/Game/bp/weapons/BP_MuzzleFlash.BP_MuzzleFlash_C" (`KismetMathLibrary.MakeTransform` _transform_location_3) "Undefined" "OverrideRootScale" null null)
            (set `self.Ammo Mag Curr` (- (`self.Ammo Mag Curr`) 1))
            (set `self.ShootDelayOver?` false)
            (`KismetSystemLibrary.K2_SetTimer` null "RememberShootDelay" (`self.Firerate`))))))))

(event `Fire`
  (set `self.IsShooting?` true)
  (set `self.Player Cam` (`/Game/bp/BP_player_char.first_person_camera` (`self.Player`)))
  (`self.Shoot`))

(event `StopFire`
  (set `self.IsShooting?` false))

(event `Reload`
  (if (and (< (`self.Ammo Mag Curr`) (`self.Ammo Mag`)) (> (`self.Ammo Current`) 0))
    (`/Game/bp/BP_player_char.Play User Animation` (`self.Player`) "reload")
    (if (>= (- (`self.Ammo Current`) (- (`self.Ammo Mag`) (`self.Ammo Mag Curr`))) 0)
      (set `self.Ammo Current` (- (`self.Ammo Current`) (- (`self.Ammo Mag`) (`self.Ammo Mag Curr`))))
      (set `self.Ammo Mag Curr` (`self.Ammo Mag`))
      (else
        (set `self.Ammo Mag Curr` (+ (`self.Ammo Current`) (`self.Ammo Mag Curr`)))
        (set `self.Ammo Current` 0)))))

(event `RememberShootDelay`
  (set `self.ShootDelayOver?` true)
  (if (and (`self.IsShooting?`) (`|EnumInequality` (`self.Firemode`) "NewEnumerator0"))
    (`self.Shoot`)))

(event `self.ReceiveBeginPlay`
  (`self.Set Weapon State` "NewEnumerator0")
  (bind _returnvalue (`|GetDataTableRow` "/Game/bp/weapons/DT_weapondata.DT_weapondata" (`KismetStringLibrary.Conv_StringToName` (`self.NAME`)))
    (:`then`
      (set `self.Firemode` (break `/Game/bp/weapons/Struct_weapondata` _returnvalue))
      (set `self.Muzzle Name` (`.muzzle_name_29_4D4074C04440D93269DBFAB3D328C74B` (break `/Game/bp/weapons/Struct_weapondata` _returnvalue)))
      (set `self.Burst Delay` (`.burst_delay_42_5F087D834EC4B4D5A240DE8F7555C7F6` (break `/Game/bp/weapons/Struct_weapondata` _returnvalue)))
      (set `self.Firerate` (`.firerate_10_B52B942A4E9E72283B2E6B8C3AD7435D` (break `/Game/bp/weapons/Struct_weapondata` _returnvalue)))
      (set `self.Velocity` (`.velocity_45_2B5E81AB40DD4A18D9D0E39CD3E1D466` (break `/Game/bp/weapons/Struct_weapondata` _returnvalue)))
      (set `self.Weapon Spread` (`.weapon_spread_39_CCB2C15F449393ACED9B9E8E03A6425C` (break `/Game/bp/weapons/Struct_weapondata` _returnvalue)))
      (set `self.Reloadelay` (`.reloadelay_11_40C95CFA41A8420032FA53B74706DA0B` (break `/Game/bp/weapons/Struct_weapondata` _returnvalue)))
      (set `self.Min Damage` (`.min_damage_15_DE0596BC426C622A82F55E8CE4038F05` (break `/Game/bp/weapons/Struct_weapondata` _returnvalue)))
      (set `self.Max Damage` (`.max_damage_16_6E4378734676E6185ED40084276612F5` (break `/Game/bp/weapons/Struct_weapondata` _returnvalue)))
      (bind _output_get (set `self.Ammo Mag` (`.ammo_mag_34_27A4BC054666F8DFC409A48004D851E5` (break `/Game/bp/weapons/Struct_weapondata` _returnvalue))))
      (set `self.Ammo All Max` (`.ammo_all_max_33_9EF0C9134737BE53E6AF538F8D7A4176` (break `/Game/bp/weapons/Struct_weapondata` _returnvalue)))
      (set `self.Ammo Current` (`.ammo_current_32_F8A53191441DB03ED1D025B59DAADB19` (break `/Game/bp/weapons/Struct_weapondata` _returnvalue)))
      (set `self.Fire Montage` (`.fire_montage_31_933C92DB43415D8A5E1CDBA3484A326C` (break `/Game/bp/weapons/Struct_weapondata` _returnvalue)))
      (set `self.Reload Montage` (`.reload_montage_30_34C099264753855159CD4097C8621497` (break `/Game/bp/weapons/Struct_weapondata` _returnvalue)))
      (set `self.Burst Amount` (`.burst_amount_48_24EC73EF46FACA5D9F4199B7CF7A40E9` (break `/Game/bp/weapons/Struct_weapondata` _returnvalue)))
      (set `self.Ammo Mag Curr` _output_get))
    (:`RowNotFound`
      (`KismetSystemLibrary.PrintString` "Weapon row not found" true true (struct :`R` 1.0 :`G` 0.036246 :`A` 1.0)))))

(event `/Game/bp/InteractionInterface.OnInteracted`
  (params (Player :type "/Game/bp/BP_player_char Object Reference"))
  (bind _currentweaponslot (`/Game/bp/BP_player_char.CurrentWeaponSlot` (`self.Player`)))
  (bind _output_get (set `self.Player` Player))
  (`/Game/bp/BP_player_char.give weapon` _output_get self)
  (`self.Set Weapon State` "NewEnumerator1")
  (set `self.MySlot` (`|GetEnumeratorNameAsString` _currentweaponslot))
  (`KismetSystemLibrary.PrintString` (`KismetStringLibrary.Concat_StrStr` (`|GetEnumeratorNameAsString` _currentweaponslot) " slot " (`self.NAME`)) true true (struct :`R` 1.0 :`G` 0.462303 :`A` 1.0)))

(fn `calc_vel_and_path`
  (returns (Transform_location :type "Vector Structure") (Velocity :type "Vector Structure") (Transform_rotation :type "Rotator Structure"))
  (bind _player_cam (`self.Player Cam`))
  (bind _returnvalue (`SceneComponent.GetSocketLocation` (`self.Weapon_mdl`) "b_gun_muzzleflash"))
  (return _returnvalue (* (`KismetMathLibrary.Normal` (- (+ (`SceneComponent.K2_GetComponentLocation` _player_cam) (* (`SceneComponent.GetForwardVector` _player_cam) 10000)) _returnvalue)) (`self.Velocity`)) (`SceneComponent.K2_GetComponentRotation` _player_cam)))

(fn `Drop`
  (`self.Set Weapon State` "NewEnumerator0"))

(fn `GetInteractionText`
  (returns (Text :type Text))
  (return "Pick Up"))

(fn `GetInteractionTxtAttach`
  (returns (AttachComponent :type "SceneComponent Object Reference"))
  (return (`self.Weapon_mdl`)))

(fn `Glow`
  (params (ON :type Boolean))
  (`PrimitiveComponent.SetRenderCustomDepth` (`self.Weapon_mdl`) ON))

(fn `Set Weapon State`
  (params (NewWeaponState :type "/Game/bp/weapons/WeaponState Enum" :default "NewEnumerator0"))
  (bind _weapon_mdl (`self.Weapon_mdl`))
  (bind _weapon_mdl_2 (`self.Weapon_mdl`))
  (bind _output_get (set `self.Weapon State` NewWeaponState))
  (switch `/Game/bp/weapons/WeaponState` _output_get
    (:`NewEnumerator0`
      (`PrimitiveComponent.SetCollisionProfileName` (`self.Sphere`) "OverlapAllDynamic" true)
      (`PrimitiveComponent.SetSimulatePhysics` _weapon_mdl true :!pinned true) ; вот тут крч вместо симулейта функцию на вращение и подсветку сделать
      (`PrimitiveComponent.SetCollisionProfileName` _weapon_mdl "WeaponDropped" true))
    (:`NewEnumerator1`
      (`PrimitiveComponent.SetCollisionProfileName` (`self.Sphere`) "NoCollision" true)
      (`PrimitiveComponent.SetSimulatePhysics` _weapon_mdl_2 false)
      (`PrimitiveComponent.SetCollisionProfileName` _weapon_mdl_2 "NoCollision" true)
      (`SceneComponent.ResetRelativeTransform` _weapon_mdl_2))))

(fn `UserConstructionScript`
  (`parent.UserConstructionScript`))