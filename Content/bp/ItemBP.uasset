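; ItemBP is an interactable item Blueprint that shows an on-screen interaction prompt when triggered by a player.
; TriggerON checks that the item overlaps the player's InteractionCube, then creates a screen-space InteractionWidget component at runtime and calls Glow.
; TriggerOFF destroys that component and turns Glow off.
; GetInteractionText and GetInteractionTxtAttach supply default text and attach point, while Glow is an empty stub.
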(event `/Game/bp/InteractionInterface.TriggerON`
  (params (Player :type "/Game/bp/BP_player_char Object Reference"))
  (if (!= (`KismetArrayLibrary.Array_Find` (`PrimitiveComponent.GetOverlappingActors` (`/Game/bp/BP_player_char.InteractionCube` Player) "/Script/Engine.Actor") self) -1)
    (`self.InteractionWidgetComponent`
      (:`then`)
      (:`else`
        (bind _returnvalue (`|CreateWidget` "/Game/bp/widgets/InteractionWidget.InteractionWidget_C" (cast `PlayerController` (`Pawn.GetController` Player) :!pure true) (`self.GetInteractionText`)))
        (bind _returnvalue_2 (`AddComponent|NODE_AddWidgetComponent-0`))
        (bind _output_get (set `self.InteractionWidgetComponent` _returnvalue_2))
        (`WidgetComponent.SetWidget` _output_get _returnvalue)
        (`WidgetComponent.SetWidgetSpace` _output_get "Screen")
        (`WidgetComponent.SetDrawAtDesiredSize` _output_get true)
        (`PrimitiveComponent.SetCollisionEnabled` _output_get "NoCollision")
        (`SceneComponent.K2_AttachToComponent` _output_get (`self.GetInteractionTxtAttach`) "None" "SnapToTarget" "SnapToTarget" "SnapToTarget" true)
        (`self.Glow` true)))))

(event `/Game/bp/InteractionInterface.TriggerOFF`
  (bind _interactionwidgetcomponent (`self.InteractionWidgetComponent`)
    (:`then`
      (`ActorComponent.K2_DestroyComponent` _interactionwidgetcomponent)
      (`self.Glow` false))
    (:`else`)))

(fn `GetInteractionText`
  (returns (Text :type Text))
  (return "Interact"))

(fn `GetInteractionTxtAttach`
  (returns (AttachComponent :type "SceneComponent Object Reference"))
  (return (`self.DefaultSceneRoot`)))

(fn `Glow`
  (params (ON :type Boolean)))

(fn `UserConstructionScript`)