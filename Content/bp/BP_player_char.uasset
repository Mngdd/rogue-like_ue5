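; Player character Blueprint handling movement, health, two-slot weapons, interaction and first/third-person camera toggling, with debug keys.
; Input drives equipped-gun actions and slot switching, which re-sockets guns to hand or back.
; An overlap cube messages InteractionInterface actors.
; Tick detects death, plays animation, blends the third-person camera toward the head via timeline, drops weapons, then respawns and possesses a new character at a hardcoded location.
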(event `self.ReceiveBeginPlay`
  ;[0.1602 1 0] BEGINPLAY
  (bind _returnvalue (`|CreateWidget` "/Game/bp/widgets/Player_UI.Player_UI_C"))
  (bind _output_get (set `self.Player_UI` _returnvalue))
  (`UserWidget.AddToViewport` _output_get 0)
  (set `/Game/bp/widgets/Player_UI.Player_var` self _output_get)
  (`self.give weapon` null))

(event `InputAxis|MoveForward`
  (params (AxisValue :type "Float (single-precision)"))
  ;[1 0.7137 0] MOVEMENT AND SPEED
  (`self.AddMovementInput` (`SceneComponent.GetForwardVector` (`self.CapsuleComponent`)) (* AxisValue (`self.MovementMultip`) (`GameplayStatics.GetWorldDeltaSeconds`)))
  (set `self.char speed` (`KismetMathLibrary.VSize` (`self.GetVelocity`)) :!label _label))

(event `InputAxis|MoveRight`
  (params (AxisValue :type "Float (single-precision)"))
  ;[1 0.7137 0] MOVEMENT AND SPEED
  (`self.AddMovementInput` (`SceneComponent.GetRightVector` (`self.CapsuleComponent`)) (* AxisValue (`self.MovementMultip`) (`GameplayStatics.GetWorldDeltaSeconds`)))
  (goto _label))

(event `InputAxis|Turn`
  (params (AxisValue :type "Float (single-precision)"))
  ;[1 0.7137 0] MOVEMENT AND SPEED
  ;;[1 1 1] ROTATION
  (`self.AddControllerYawInput` (* AxisValue (`self.MouseSens`))))

(event `InputAction|DEBUG_HPDAMAGE`
  (params (Key :type "Key Structure"))
  ;[0.6317 1 0.8236] DEBUG (debug heal -> alt + H, damage -> alt + K, switch cam view -> B, K -> suicide)
  (:`Pressed`
    (set `self.Health` (- (`self.Health`) 10))))

(event `Key|B`
  (params (Key :type "Key Structure"))
  ;[0.6317 1 0.8236] DEBUG (debug heal -> alt + H, damage -> alt + K, switch cam view -> B, K -> suicide)
  (:`Pressed`
    (`/Engine/EditorBlueprintResources/StandardMacros.FlipFlop`
      (:`A`
        (`self.Switch Cams` (`self.third_person_camera`) (`self.first_person_camera`)))
      (:`B`
        (`self.Switch Cams` (`self.first_person_camera`) (`self.third_person_camera`))))))

(event `InputAction|Reload`
  (params (Key :type "Key Structure"))
  ;[1 1 1] Reload
  (:`Pressed`
    (bind _returnvalue (`self.EquippedGun`)
      (:`Is Valid`
        (`/Game/bp/weapons/BaseWeaonBP.Reload` _returnvalue)))))

(event `Key|K`
  (params (Key :type "Key Structure"))
  ;[0.6317 1 0.8236] DEBUG (debug heal -> alt + H, damage -> alt + K, switch cam view -> B, K -> suicide)
  (:`Pressed`
    (`self.player_hp_changer` -1000000)))

(event `InputAction|fire`
  (params (Key :type "Key Structure"))
  ;[1 1 1] shoot
  (:`Pressed`
    (bind _returnvalue (`self.EquippedGun`)
      (:`Is Valid`
        (`/Game/bp/weapons/BaseWeaonBP.Fire` _returnvalue))))
  (:`Released`
    (bind _returnvalue_2 (`self.EquippedGun`)
      (:`Is Valid`
        (`/Game/bp/weapons/BaseWeaonBP.StopFire` _returnvalue_2)))))

(event `InputAction|DEBUG_HPHEAL`
  (params (Key :type "Key Structure"))
  ;[0.6317 1 0.8236] DEBUG (debug heal -> alt + H, damage -> alt + K, switch cam view -> B, K -> suicide)
  (:`Pressed`
    (`self.player_hp_changer` 0)))

(event `self.InteractionCube.OnComponentBeginOverlap`
  (params (OverlappedComponent :type "PrimitiveComponent Object Reference") (OtherActor :type "Actor Object Reference") (OtherComp :type "PrimitiveComponent Object Reference") (OtherBodyIndex :type Integer) (bFromSweep :type Boolean) (SweepResult :type "HitResult Structure (by ref)"))
  ;[1 0.5558 0.1823] TRIGGER ON/OFF INTERACTION INTERFACE
  (if (`KismetSystemLibrary.DoesImplementInterface` OtherActor "/Game/bp/InteractionInterface.InteractionInterface_C")
    (message `/Game/bp/InteractionInterface.TriggerON` OtherActor self)))

(event `InputAction|Switch`
  (params (Key :type "Key Structure"))
  ;[1 1 1] switch weapons
  (:`Pressed`
    (switch `/Game/bp/weapons/WeaponSlots` (`self.CurrentWeaponSlot`)
      (:`NewEnumerator0`
        (set `self.CurrentWeaponSlot` "NewEnumerator1"))
      (:`NewEnumerator1`
        (set `self.CurrentWeaponSlot` "NewEnumerator0")))
    (`self.switch_weapon`)))

(event `self.InteractionCube.OnComponentEndOverlap`
  (params (OverlappedComponent :type "PrimitiveComponent Object Reference") (OtherActor :type "Actor Object Reference") (OtherComp :type "PrimitiveComponent Object Reference") (OtherBodyIndex :type Integer))
  ;[1 0.5558 0.1823] TRIGGER ON/OFF INTERACTION INTERFACE
  (if (`KismetSystemLibrary.DoesImplementInterface` OtherActor "/Game/bp/InteractionInterface.InteractionInterface_C")
    (message `/Game/bp/InteractionInterface.TriggerOFF` OtherActor)))

(event `InputAction|Interact`
  (params (Key :type "Key Structure"))
  ;[1 0.5486 0.166] Interaction -> E
  (:`Pressed`
    (for _array_element (`PrimitiveComponent.GetOverlappingActors` (`self.InteractionCube`) "/Script/Engine.Actor")
      (if (`KismetSystemLibrary.DoesImplementInterface` _array_element "/Game/bp/InteractionInterface.InteractionInterface_C")
        (message `/Game/bp/InteractionInterface.OnInteracted` _array_element self)
        (break)))))

(event `self.ReceiveTick`
  (params (DeltaSeconds :type "Float (single-precision)"))
  (bind _death_cam (`self.death_Cam`))
  (bind _primaryweapon (`self.PrimaryWeapon`))
  (bind _secondaryweapon (`self.SecondaryWeapon`))
  (bind _third_person_camera (`self.third_person_camera`))
  ;[1 1 1] HP
  (bind _output_get (set `self.HealtProcent` (/ (`self.Health`) 100.0)))
  (if (and (not (`self.died`)) (<= _output_get 0.0))
    (set `self.died` true)
    ;[1 0.1067 0] DEATH (MAKE SPAWNPOINTS)
    (`SkeletalMeshComponent.PlayAnimation` (`self.Mesh`) "/Game/Anims/AnimStarterPack/Death_1.Death_1" false)
    (`self.DisableInput` (`GameplayStatics.GetPlayerController` 0))
    (`SceneComponent.K2_DetachFromComponent` _death_cam "KeepWorld" "KeepWorld" "KeepWorld" true)
    (set `self.fpp_pos` (`SceneComponent.GetRelativeTransform` _death_cam))
    (`SceneComponent.K2_AttachToComponent` _death_cam (`self.Mesh`) "headSocket" "KeepWorld" "KeepWorld" "KeepWorld" true)
    (`SceneComponent.K2_DetachFromComponent` _third_person_camera "KeepWorld" "KeepWorld" "KeepWorld" true)
    (set `self.tpp_pos` (`SceneComponent.GetRelativeTransform` _third_person_camera))
    (bind (_direction _cam_track) (`Timeline|Timeline_1`)
      (:`Update`
        (bind _returnvalue (`KismetMathLibrary.TLerp` (`self.tpp_pos`) (`self.fpp_pos`) _cam_track))
        (`SceneComponent.K2_SetRelativeTransform` (`self.third_person_camera`) (`KismetMathLibrary.MakeTransform` (.location _returnvalue) (`KismetMathLibrary.MakeRotator` 0.0 (.pitch (.rotation _returnvalue)) (.yaw (.rotation _returnvalue))) (.scale _returnvalue)) false false)
        (`Controller.SetControlRotation` (`GameplayStatics.GetPlayerController` 0) (`KismetMathLibrary.MakeRotator` 0.0 0.0 (.yaw (.rotation _returnvalue)))))
      (:`Finished`
        (`/Engine/EditorBlueprintResources/StandardMacros.IsValid` _primaryweapon
          (:`Is Valid`
            (`/Game/bp/weapons/BaseWeaonBP.Drop` _primaryweapon))
          (:`Is Not Valid`
            _))
        (`/Engine/EditorBlueprintResources/StandardMacros.IsValid` _secondaryweapon
          (:`Is Valid`
            (`/Game/bp/weapons/BaseWeaonBP.Drop` _secondaryweapon))
          (:`Is Not Valid`
            _))
        (`KismetSystemLibrary.Delay` 5.0)
        (`self.K2_DestroyActor` (`GameplayStatics.GetPlayerCharacter` 0))
        (`self.EnableInput` (`GameplayStatics.GetPlayerController` 0))
        (bind _returnvalue_2 (`|SpawnActorFromClass` "BP_player_char_C" (`KismetMathLibrary.MakeTransform` (656.107544 -474.044678 269.03595)) "Undefined" "OverrideRootScale" null null))
        (`Controller.Possess` (`GameplayStatics.GetPlayerController` 0) _returnvalue_2)))))

(fn `give weapon`
  (params (Weapon :type "/Game/bp/weapons/BaseWeaonBP Object Reference"))
  (`/Engine/EditorBlueprintResources/StandardMacros.IsValid` (`self.PrimaryWeapon`) ; если первый слот не существуеэ, то суем туды
    (:`Is Valid`
      (`/Engine/EditorBlueprintResources/StandardMacros.IsValid` (`self.SecondaryWeapon`)
        (:`Is Valid`
          (bind _returnvalue (`self.EquippedGun`)
            (:`Is Valid`
              (`self.K2_DetachFromActor` _returnvalue "KeepWorld" "KeepWorld" "KeepWorld")
              (`/Game/bp/weapons/BaseWeaonBP.Drop` _returnvalue)
              (`self.SetEquippedGun` null)
              (`self.give weapon` (`local.Weapon`)))))
        (:`Is Not Valid`
          (set `self.SecondaryWeapon` (`local.Weapon`))
          (`self.switch_weapon` :!label _label))))
    (:`Is Not Valid`
      (set `self.PrimaryWeapon` (`local.Weapon`))
      (goto _label))))

(fn `Play User Animation`
  (params (AnimName :type String))
  (bind (_value _returnvalue) (`BlueprintMapLibrary.Map_Find` (`self.AnimDict`) AnimName))
  (if _returnvalue
    (`self.PlayAnimMontage` _value)
    (else
      (`KismetSystemLibrary.PrintString` (`KismetStringLibrary.Concat_StrStr` "NO ANIMATION CALLED " AnimName) true true (struct :`R` 1.0 :`A` 1.0)))))

(fn `player_hp_changer`
  (params (`hp_+-` :type Integer))
  (returns (hp_amount :type Integer))
  (bind _output_get (set `self.Health` (+ (`self.Health`) `hp_+-`)))
  (return _output_get))

(fn `Switch Cams`
  (params (from :type "CameraComponent Object Reference") (to :type "CameraComponent Object Reference"))
  (`ActorComponent.SetActive` from false false)
  (`ActorComponent.SetActive` to true false))

(fn `switch_weapon`
  (`|ExecutionSequence`
    (:`then_0`
      (bind _returnvalue (`self.EquippedGun`)
        (:`Is Valid`
          (`self.K2_AttachToComponent` _returnvalue (`self.Mesh`) "skt_rhand" "SnapToTarget" "SnapToTarget" "SnapToTarget" true))))
    (:`then_1`
      (bind _returnvalue_2 (`self.StowedGun`) ; stowed gun - сложенное оружие
        (:`Is Valid`
          (`self.K2_AttachToComponent` _returnvalue_2 (`self.Mesh`) "skt_back" "SnapToTarget" "SnapToTarget" "SnapToTarget" true))))))

(fn `UserConstructionScript`)